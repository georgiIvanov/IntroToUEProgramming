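; MyCharacter is a character Blueprint with a power level that battery power can raise and that is reflected in its mesh material.
; The PowerUp event adds the battery amount by interpolating from the current level to the new total along a timeline curve.
; Construction creates a dynamic material and records the initial power level.
; Tick feeds the ratio of current to initial power into the material's PowerMultiplier parameter.
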(event `self.PowerUp`
  (params (BatteryPower :type "Float (single-precision)"))
  (bind _powerlevel (`self.PowerLevel`))
  (set `self.PreChargePowerLevel` _powerlevel)
  (set `self.ResultingPowerLevel` (+ BatteryPower _powerlevel))
  (bind (_direction _powerupcurve) (`Timeline|PowerUpTimeline` :!via `PlayFromStart`)
    (:`Update`
      (set `self.PowerLevel` (`KismetMathLibrary.Lerp` (`self.PreChargePowerLevel`) (`self.ResultingPowerLevel`) _powerupcurve)))))

(event `self.ReceiveTick`
  (params (DeltaSeconds :type "Float (single-precision)"))
  (`parent.ReceiveTick` DeltaSeconds)
  (`MaterialInstanceDynamic.SetScalarParameterValue` (`self.Dynamic Power Material`) "PowerMultiplier" (/ (`self.PowerLevel`) (`self.Initial Power Level`))))

(fn `UserConstructionScript`
  (bind _returnvalue (`PrimitiveComponent.CreateDynamicMaterialInstance` (`self.Mesh`) 0 null))
  (set `self.Dynamic Power Material` _returnvalue)
  (set `self.Initial Power Level` (`self.PowerLevel`)))